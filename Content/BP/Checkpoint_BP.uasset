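; Checkpoint actor that saves the player's location or clears the saved checkpoint when its Trigger is overlapped, depending on its Load flag.
; With Load on, it stores the ThirdPersonCharacter's location and a load flag in the "Check" slot, reusing or creating a Save_loc object.
; With Load off, any overlapping actor switches off the load flag in the existing save.
; Debug prints report both outcomes.
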(event `self.Trigger.OnComponentBeginOverlap`
  (params (OverlappedComponent :type "PrimitiveComponent Object Reference") (OtherActor :type "Actor Object Reference") (OtherComp :type "PrimitiveComponent Object Reference") (OtherBodyIndex :type Integer) (bFromSweep :type Boolean) (SweepResult :type "HitResult Structure (by ref)"))
  (bind _player_location (`self.Player_location`))
  (if (`self.Load`)
    (bind _asthird_person_character (cast `/Game/BP/ThirdPersonBP/Blueprints/ThirdPersonCharacter` OtherActor))
    (`|ExecutionSequence`
      (:`then_0`
        ;[1 1 1] Hitta spelarens location
        (if true
          (set `self.Player_location` (`self.K2_GetActorLocation` _asthird_person_character))
          (`KismetSystemLibrary.PrintString` "SAVED")))
      (:`then_1`
        (bind _returnvalue (`GameplayStatics.DoesSaveGameExist` "Check"))
        (if _returnvalue
          ;[1 1 1] If "game save exist" ladda variablarna och spara dom
          (bind _returnvalue_2 (`GameplayStatics.LoadGameFromSlot` "Check"))
          (bind _assave_loc (cast `/Game/BP/Save_loc` _returnvalue_2))
          (set `/Game/BP/Save_loc.Player_location` _player_location _assave_loc)
          (set `/Game/BP/Save_loc.Load` true _assave_loc)
          (`GameplayStatics.SaveGameToSlot` _assave_loc "Check")
          (else
            ;[1 1 1] Om flask så skapar den en ny istället
            (bind _returnvalue_3 (`GameplayStatics.CreateSaveGameObject` "/Game/BP/Save_loc.Save_loc_C"))
            (set `/Game/BP/Save_loc.Player_location` _player_location _returnvalue_3)
            (set `/Game/BP/Save_loc.Load` true _returnvalue_3)
            (`GameplayStatics.SaveGameToSlot` _returnvalue_3 "Check")))))
    (else
      ;[1 1 1] If loading is turned off, then load the game and turn off loading within our save
      (bind _returnvalue_4 (`GameplayStatics.LoadGameFromSlot` "Check"))
      (bind _assave_loc_2 (cast `/Game/BP/Save_loc` _returnvalue_4))
      (set `/Game/BP/Save_loc.Load` false _assave_loc_2)
      (`GameplayStatics.SaveGameToSlot` _assave_loc_2 "Check")
      (`KismetSystemLibrary.PrintString` "Checkpoint cleared"))))

(fn `UserConstructionScript`)