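; BP_Spider is an enemy spider that attacks its Target and can send the player back to a checkpoint.
; Tick checks range and montage state, then briefly deactivates CharacterMovement and plays the attack montage.
; As the montage starts, movement reactivates and a DeathBox overlap moves the player to the "Check" save's location, or opens a level without one.
; Chase logic is absent here; the AIMoveTo chain is unused.
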(event `self.ReceiveBeginPlay`
  (set `CharacterMovementComponent.MaxWalkSpeed` (`self.WalkingSpeed`) (`self.CharacterMovement`)))

(event `self.ReceiveTick`
  (params (DeltaSeconds :type "Float (single-precision)"))
  ;[1 1 1] Stops attack & movement if attacking
  (if (and (`self.Is Within Attack Range`) (not (`self.Is Attacking`)))
    (`self.Deactivate AI Movement`)
    (`|PlayMontage` (`self.Mesh`) "/Game/Characters/Enemy_Great_Spider/Animations/SpiderAttack2.SpiderAttack2"
      (:`then`
        (if (`PrimitiveComponent.IsOverlappingActor` (`self.DeathBox`) (`self.Target`))
          (`self.Activate AI Movement`)
          (cast `/Game/BP/ThirdPersonBP/Blueprints/ThirdPersonCharacter` (`self.Target`))
          (bind _returnvalue (`GameplayStatics.DoesSaveGameExist` "Check"))
          (if _returnvalue
            (bind _returnvalue_2 (`GameplayStatics.LoadGameFromSlot` "Check"))
            (bind _assave_loc (cast `/Game/BP/Save_loc` _returnvalue_2))
            (bind _asthird_person_character (cast `/Game/BP/ThirdPersonBP/Blueprints/ThirdPersonCharacter` (`self.Target`)))
            (`self.K2_SetActorLocation` _asthird_person_character (`/Game/BP/Save_loc.Player_location` _assave_loc) false false)
            (else
              (`GameplayStatics.OpenLevel` (`self.Level`))))
          (else
            (`self.Activate AI Movement`)))))))

(event `SpiderGetDoll_1`
  (params (Doll :type "Actor Object Reference")))

(fn `Activate AI movement`
  (`ActorComponent.Activate` (`self.CharacterMovement`) false))

(fn `Deactivate AI Movement`
  (`ActorComponent.Deactivate` (`self.CharacterMovement`)))

(fn `Is Attacking`
  (returns (ReturnValue :type Boolean))
  ;[1 1 1] Checks if attack montage is playing
  (return (`AnimInstance.Montage_IsPlaying` (`SkeletalMeshComponent.GetAnimInstance` (`self.Mesh`)) "/Game/Characters/Enemy_Great_Spider/Animations/SpiderAttack2.SpiderAttack2")))

(fn `Is Within Attack Range`
  (returns (ReturnValue :type Boolean))
  ;[1 1 1] checks range to player character
  (return (< (`self.GetDistanceTo` (`self.Target`) self) (`self.Attack Range`))))

(fn `UserConstructionScript`)