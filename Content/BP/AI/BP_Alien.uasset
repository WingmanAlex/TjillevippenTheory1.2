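; BP_Alien is an enemy AI character that chases the player marine and attacks in melee.
; While alive it repeats AI MoveTo; Tick plays the attack montage when in range, pausing movement until it completes.
; AnyDamage lowers health; at zero it disables movement and collision, credits the marine's kill, notifies the game mode, then destroys itself after a delay.
; It registers with the game mode for scaling and exposes DamagePlayer for applying hits.
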(event `self.ReceiveBeginPlay`
  ;[1 1 1] Reference to Alien Scaling
  (message `/Game/BluePrints/Interfaces/BP_Interface.Get Reference Scale Alien` (`GameplayStatics.GetGameMode`) self)
  ;[1 1 1] Only alows Movement if not dead
  (if (`self.Is Alive`) :!label _label
    ;[1 1 1] AI move to player + repeat
    (`|AIMoveTo` self (0.0 0.0 0.0) (`GameplayStatics.GetPlayerCharacter` 0)
      (:`OnSuccess`
        _)
      (:`OnFail`
        _))
    (`KismetSystemLibrary.Delay` 0.2)
    (goto _label)))

(event `/Game/BluePrints/Interfaces/BP_Interface.Scale Aliens`
  ;[1 1 1] Increases Alien size
  (`self.SetActorScale3D` (2.0 2.0 2.0)))

(event `self.ReceiveTick`
  (params (DeltaSeconds :type "Float (single-precision)"))
  ;[1 1 1] Update if alien in range, If alien is not attacking play attack anim montage, deactivate movement when attacking & move again
  (if (`self.Can Attack`)
    (`self.Deactivate AI Movement`)
    (`|PlayMontage` (`self.Mesh`) "/Game/Characters/Enemy_Great_Spider/Animations/AlienAttack1.AlienAttack1"
      (:`OnCompleted`
        (`self.Activate AI movement`)))))

(event `self.ReceiveAnyDamage`
  (params (Damage :type "Float (single-precision)") (DamageType :type "DamageType Object Reference") (InstigatedBy :type "Controller Object Reference") (DamageCauser :type "Actor Object Reference"))
  ;[1 1 1] Decreases Alien Health on DMG, if health == 0 AI get killed and destroyed
  (if (`self.Is Alive`)
    (bind _health (`self.Decrease Health` Damage))
    (if (== _health 0.0)
      (`self.Kill AI`)
      (`KismetSystemLibrary.Delay` 3.0)
      (`self.K2_DestroyActor`))))

(fn `Activate AI movement`
  (`ActorComponent.Activate` (`self.CharacterMovement`) false))

(fn `Can Attack`
  (returns (ReturnValue :type Boolean))
  ;[1 1 1] Checks if alien is within attack range to marine, alive and if its currently attacking
  (return (and (`self.Is Within Attack Range`) (not (`self.Is Attacking`)) (`self.Is Alive`))))

(fn `Damage Player`
  ;[1 1 1] Applies DMG on PC if alive
  (if (`self.Is Alive`)
    (`GameplayStatics.ApplyDamage` (`GameplayStatics.GetPlayerCharacter` 0) (`self.Damage Per Hit`))))

(fn `Deactivate AI Movement`
  (bind _charactermovement (`self.CharacterMovement`))
  ;[1 1 1] deactivate AI movement
  (`MovementComponent.StopMovementImmediately` _charactermovement)
  (`ActorComponent.Deactivate` _charactermovement))

(fn `Decrease Health`
  (params (`Damage Amount` :type "Float (double-precision)"))
  (returns (Health :type "Float (double-precision)"))
  ;[1 1 1] Alien health decrease from damage amount
  (bind _output_get (set `self.Health` (`KismetMathLibrary.FClamp` (- (`self.Health`) `Damage Amount`) 0.0 100.0)))
  (return _output_get))

(fn `Is Alive`
  (returns (ReturnValue :type Boolean))
  ;[1 1 1] returns if alien is alive
  (return (not (`self.Dead`))))

(fn `Is Attacking`
  (returns (ReturnValue :type Boolean))
  ;[1 1 1] Checks if anim montage is playing
  (return (`AnimInstance.Montage_IsPlaying` (`SkeletalMeshComponent.GetAnimInstance` (`self.Mesh`)) "/Game/Characters/Enemy_Great_Spider/Animations/AlienAttack1.AlienAttack1")))

(fn `Is Within Attack Range`
  (returns (ReturnValue :type Boolean))
  ;[1 1 1] Distance to PC &
  (return (< (`self.GetDistanceTo` (`GameplayStatics.GetPlayerCharacter` 0)) (`self.Attack Range`))))

(fn `Kill AI`
  ;[1 1 1] If AI is Dead deactivate Movement & zero collision
  (set `self.Dead` true)
  (`self.Deactivate AI Movement`)
  (`self.SetActorEnableCollision` false)
  ;[1 1 1] Increases kill count on alien death
  (bind _asbp_marine (cast `/Game/BluePrints/Pawns/BP_Marine` (`GameplayStatics.GetPlayerCharacter` 0)))
  (`/Game/BluePrints/Pawns/BP_Marine.Increase Kills` _asbp_marine)
  ;[1 1 1] Register Alien death in game mode
  (bind _asbp_mars_marine_game_mode (cast `/Game/BluePrints/GameMode/BP_MarsMarine_GameMode` (`GameplayStatics.GetGameMode`)))
  (`/Game/BluePrints/GameMode/BP_MarsMarine_GameMode.Register Alien Death` _asbp_mars_marine_game_mode self))

(fn `UserConstructionScript`)