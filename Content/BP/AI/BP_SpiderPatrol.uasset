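; Spider enemy character that patrols three waypoint actors in a loop, pausing at each, and attacks the Doll player when in range.
; Tick checks distance and montage state, deactivates movement, then starts the attack montage.
; Movement reactivates as soon as the montage starts, and a Doll overlapping DeathBox is teleported to its checkpoint.
; An unconnected branch holds an alternative save-game respawn or level reload.
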(event `self.ReceiveBeginPlay`
  ;[1 1 1] Coordinate patrol for spiders
  (set `CharacterMovementComponent.MaxWalkSpeed` (`self.WalkingSpeed`) (`self.CharacterMovement`))
  (`self.Patrol`))

(event `Patrol`
  ;[1 1 1] Coordinate patrol for spiders
  (`|AIMoveTo` self (0.0 0.0 0.0) (`self.Waypoint1`) 1.0 :!label _label
    (:`OnSuccess`
      (`KismetSystemLibrary.Delay` (`self.Duration`))
      (`|AIMoveTo` self (0.0 0.0 0.0) (`self.Waypoint2`) 1.0
        (:`OnSuccess`
          (`KismetSystemLibrary.Delay` (`self.Duration`))
          (`|AIMoveTo` self (0.0 0.0 0.0) (`self.Waypoint3`) 1.0
            (:`OnSuccess`
              (`KismetSystemLibrary.Delay` (`self.Duration`))
              (goto _label))))))))

(event `self.ReceiveTick`
  (params (DeltaSeconds :type "Float (single-precision)"))
  ;[1 1 1] Stops attack & movement if attacking
  (if (and (`self.Is Within Attack Range`) (not (`self.Is Attacking`)))
    (`self.Deactivate AI movement`)
    (`|PlayMontage` (`self.Mesh`) "/Game/Characters/Enemy_Great_Spider/Animations/SpiderAttack2.SpiderAttack2"
      (:`then`
        (bind _asthird_person_character (cast `/Game/BP/ThirdPersonBP/Blueprints/ThirdPersonCharacter` (`self.Doll`)))
        (if (`PrimitiveComponent.IsOverlappingActor` (`self.DeathBox`) (`self.doll`))
          (`self.Activate AI Movement`)
          (`self.K2_SetActorLocation` (`self.Doll`) (`/Game/BP/ThirdPersonBP/Blueprints/ThirdPersonCharacter.CheckPoint` _asthird_person_character) false false)
          (else
            (`self.Activate AI Movement`)))))))

(fn `Activate AI Movement`
  (`ActorComponent.Activate` (`self.CharacterMovement`) false))

(fn `Deactivate AI Movement`
  (`ActorComponent.Deactivate` (`self.CharacterMovement`)))

(fn `Is Attacking`
  (returns (ReturnValue :type Boolean))
  (return (`AnimInstance.Montage_IsPlaying` (`SkeletalMeshComponent.GetAnimInstance` (`self.Mesh`)) "/Game/Characters/Enemy_Great_Spider/Animations/SpiderAttack2.SpiderAttack2")))

(fn `Is WIthin Attack Range`
  (returns (ReturnValue :type Boolean))
  (return (< (`self.GetDistanceTo` (`self.Doll`) self) (`self.Attack Range`))))

(fn `UserConstructionScript`)